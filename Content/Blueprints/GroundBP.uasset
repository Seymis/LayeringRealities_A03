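; Ground actor that shifts its terrain between dry and wet grass looks based on the IsRaining flag.
; BeginPlay creates a dynamic instance of MI_DryGrass, then it and every Tick check the flag.
; Rain plays the Dry2Wet timeline, while no rain plays Wet2Dry through a DoOnce that re-arms when Dry2Wet finishes.
; Both timelines drive the material's Wet scalar parameter.
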(event `self.ReceiveBeginPlay`
  (bind _terrain (`self.Terrain`))
  (`PrimitiveComponent.CreateDynamicMaterialInstance` (`self.Terrain`) 0 "/Game/Models/MI_DryGrass.MI_DryGrass" "None")
  (if (`self.Is Raining?`) :!label _label
    (bind (_direction _wetness) (`Timeline|Dry2Wet`)
      (:`Update`
        (`MeshComponent.SetScalarParameterValueOnMaterials` _terrain "Wet" _wetness))
      (:`Finished`
        (goto _label_2 :!via `Reset`)))
    (else
      (`/Engine/EditorBlueprintResources/StandardMacros.DoOnce` true :!label _label_2
        (:`Completed`
          (bind (_direction_2 _wetness_2) (`Timeline|Wet2Dry`)
            (:`Update`
              _)
            (:`Finished`
              _))
          (`MeshComponent.SetScalarParameterValueOnMaterials` _terrain "Wet" _wetness_2))))))

(event `self.ReceiveTick`
  (params (DeltaSeconds :type "Float (single-precision)"))
  (goto _label))

(fn `UserConstructionScript`)