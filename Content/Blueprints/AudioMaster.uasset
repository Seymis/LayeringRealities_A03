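; AudioMaster is an actor that crossfades between rain audio and base ambient audio according to IsRaining.
; Tick polls the flag, with DoOnce gates keeping each branch from respawning its sound every frame.
; Each transition spawns and fades in its sound at world origin, then fades out the other after a delay.
; The rain branch re-arms the base-audio gate, but nothing resets the rain gate.
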(event `self.ReceiveBeginPlay`)

(event `self.ReceiveTick`
  (params (DeltaSeconds :type "Float (single-precision)"))
  (if (`self.Is Raining?`)
    (`/Engine/EditorBlueprintResources/StandardMacros.DoOnce` false
      (:`Completed`
        (`|ExecutionSequence`
          (:`then_0`
            (bind _returnvalue (`GameplayStatics.SpawnSoundAtLocation` "/Game/Audio/Rainm_mixdown.Rainm_mixdown" (0.0 0.0 0.0) (struct) 1.0 1.0 0.0 null null))
            (`AudioComponent.FadeIn` _returnvalue 2.0 1.0 0.0 "Linear")
            (`KismetSystemLibrary.Delay` 2.0)
            (`AudioComponent.FadeOut` (stale _returnvalue_2) 6.0 0.0 "Linear"))
          (:`then_1`
            (goto _label :!via `Reset`)))))
    (else
      (`/Engine/EditorBlueprintResources/StandardMacros.DoOnce` false :!label _label
        (:`Completed`
          (bind _returnvalue_2 (`GameplayStatics.SpawnSoundAtLocation` "/Game/Audio/BAseAudio.BAseAudio" (0.0 0.0 0.0) (struct) 1.0 1.0 0.0 null null))
          (`AudioComponent.FadeIn` _returnvalue_2 2.0 1.0 0.0 "Linear")
          (`KismetSystemLibrary.Delay` 2.0)
          (`AudioComponent.FadeOut` _returnvalue 2.0 0.0 "Linear"))))))

(fn `UserConstructionScript`)