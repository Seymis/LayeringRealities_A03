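; Weather controller Blueprint that drives rain transitions through the Grasses, RainDrops and Clouds Material Parameter Collections.
; Tick checks IsRaining: one timeline plays while raining, and a DoOnce-gated second timeline plays when it is not.
; Both animate grass wind and dryness, raindrop wetness and storm clouds, each rewinding the other on finish.
; SetWindPower is an empty stub, and SetWetDry only zeroes grass Dry.
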(event `self.ReceiveBeginPlay`)

(event `self.ReceiveTick`
  (params (DeltaSeconds :type "Float (single-precision)"))
  (bind _raindrops (`self.RainDrops`))
  (bind _grasses (`self.Grasses`))
  (bind _grasses_2 (`self.Grasses`))
  (if (`self.Is Raining?`)
    (bind (_direction _wetness _wind _green _cloud) (`Timeline|Timeline_0` :!label _label)
      (:`Update`
        (`|ExecutionSequence`
          (:`then_0`
            (`KismetMaterialLibrary.SetScalarParameterValue` _grasses_2 (`self.Wind`) _wind))
          (:`then_1`
            (`KismetMaterialLibrary.SetScalarParameterValue` _grasses_2 (`self.Dry`) _green))
          (:`then_2`
            (`KismetMaterialLibrary.SetScalarParameterValue` _raindrops (`self.RainDropOff`) _wetness))
          (:`then_3`
            (`KismetMaterialLibrary.SetScalarParameterValue` (`self.Clouds`) (`self.StormClouds`) _cloud))))
      (:`Finished`
        (`|ExecutionSequence`
          (:`then_0`
            (bind (_direction_2 _wetness_2 _wind_2 _green_2 _cloud_2) (`Timeline|Timeline` :!via `SetNewTime` :!label _label_2)
              (:`Update`
                (`|ExecutionSequence`
                  (:`then_0`
                    (`KismetMaterialLibrary.SetScalarParameterValue` _grasses (`self.Wind`) _wind_2))
                  (:`then_1`
                    (`KismetMaterialLibrary.SetScalarParameterValue` _grasses (`self.Dry`) _green_2))
                  (:`then_2`
                    (`KismetMaterialLibrary.SetScalarParameterValue` _raindrops (`self.RainDropOff`) _wetness_2))
                  (:`then_3`
                    (`KismetMaterialLibrary.SetScalarParameterValue` (`self.Clouds`) (`self.StormClouds`) _cloud_2))))
              (:`Finished`
                (set `self.Start Closed` true)
                (goto _label :!via `SetNewTime`))))
          (:`then_1`
            (goto _label_3 :!via `Reset`)))))
    (else
      (`/Engine/EditorBlueprintResources/StandardMacros.DoOnce` (`self.Start Closed`) :!label _label_3
        (:`Completed`
          (goto _label_2))))))

(fn `Set Wet/Dry`
  (`KismetMaterialLibrary.SetScalarParameterValue` "/Game/Models/Grasses.Grasses" "Dry"))

(fn `Set WindPower`)

(fn `UserConstructionScript`)