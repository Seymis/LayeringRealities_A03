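; Rain controller Blueprint that drives the spawn rate of a Niagara rain effect based on the IsRaining flag.
; BeginPlay and Tick both check the flag, and while it is true a Timeline feeds its Alpha into User_SpRate.
; When false, a DoOnce gate plays a second Timeline on the same parameter.
; The first Timeline's finish resets that gate, and the second's finish sets StartClosed.
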(event `self.ReceiveBeginPlay`
  (bind _raincontroller (`self.RainController`))
  (if (`self.Is Raining?`) :!label _label
    (bind (_direction _alpha) (`Timeline|Timeline`)
      (:`Update`
        (`NiagaraComponent.SetNiagaraVariableFloat` _raincontroller "User_SpRate" _alpha))
      (:`Finished`
        (goto _label_2 :!via `Reset`)))
    (else
      (`/Engine/EditorBlueprintResources/StandardMacros.DoOnce` (`self.Start Closed`) :!label _label_2
        (:`Completed`
          (bind (_direction_2 _alpha_2) (`Timeline|Timeline_0`)
            (:`Update`
              (`NiagaraComponent.SetNiagaraVariableFloat` _raincontroller "User_SpRate" _alpha_2))
            (:`Finished`
              (set `self.Start Closed` true))))))))

(event `self.ReceiveTick`
  (params (DeltaSeconds :type "Float (single-precision)"))
  (goto _label))

(fn `UserConstructionScript`)