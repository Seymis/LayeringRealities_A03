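; Grass material manager actor that shifts a foliage mesh's wind strength and wetness with the IsRaining flag.
; BeginPlay creates a dynamic instance of the dry wild-grass material, and both it and Tick check the flag.
; Rain plays a timeline driving both scalar parameters; its completion resets a DoOnce.
; When rain is off, that DoOnce gates a second timeline driving the same parameters.
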(event `self.ReceiveBeginPlay`
  (bind _sm_vdilbaiia_varg (`self.SM_vdilbaiia_VarG`))
  (`PrimitiveComponent.CreateDynamicMaterialInstance` _sm_vdilbaiia_varg 0 "/Game/Fab/Megascans/Plants/Wild_Grass_vdilbaiia/Medium/MI_WildMainDry.MI_WildMainDry" "None")
  (if (`self.Is Raining?`) :!label _label
    (bind (_direction _wetness _wind) (`Timeline|Timeline`)
      (:`Update`
        (`|ExecutionSequence`
          (:`then_0`
            (`MeshComponent.SetScalarParameterValueOnMaterials` _sm_vdilbaiia_varg "Local Primary Wind Strength" _wind))
          (:`then_1`
            (`MeshComponent.SetScalarParameterValueOnMaterials` _sm_vdilbaiia_varg "Wet " _wetness))))
      (:`Finished`
        (goto _label_2 :!via `Reset`)))
    (else
      (`/Engine/EditorBlueprintResources/StandardMacros.DoOnce` true :!label _label_2
        (:`Completed`
          (bind (_direction_2 _wetness_2 _wind_2) (`Timeline|Timeline_0`)
            (:`Update`
              _)
            (:`Finished`
              _))
          (`|ExecutionSequence`
            (:`then_0`
              (`MeshComponent.SetScalarParameterValueOnMaterials` _sm_vdilbaiia_varg "Local Primary Wind Strength" _wind_2))
            (:`then_1`
              (`MeshComponent.SetScalarParameterValueOnMaterials` _sm_vdilbaiia_varg "Wet" _wetness_2))))))))

(event `self.ReceiveTick`
  (params (DeltaSeconds :type "Float (single-precision)"))
  (goto _label))

(fn `UserConstructionScript`)